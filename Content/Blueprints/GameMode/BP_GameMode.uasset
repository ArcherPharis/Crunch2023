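; Game mode that provides a hit pause effect by briefly changing global time dilation.
; DoHitPause applies the TimeDilation value, waits through a very short Delay, then restores normal speed.
; It only triggers at normal time speed and below the MaxHitPause limit, tracked by a counter that rises on start and falls on restore.
; The Delay runs in dilated game time, so its real length scales with the dilation.
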(event `DoHitPause`
  (if (and (== (`GameplayStatics.GetGlobalTimeDilation`) 1.0) (< (`self.hitPauseCount`) (`self.maxHitPause`)))
    (set `self.hitPauseCount` (+ (`self.hitPauseCount`) 1))
    (`GameplayStatics.SetGlobalTimeDilation` (`self.Time Dilation`))
    (`KismetSystemLibrary.Delay` 0.011)
    (`GameplayStatics.SetGlobalTimeDilation` 1.0)
    (set `self.hitPauseCount` (`KismetMathLibrary.Clamp` (- (`self.hitPauseCount`) 1) 0 (`self.maxHitPause`)))))

(fn `UserConstructionScript`)