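; GA_GroundBlast is a player gameplay ability that blasts characters at a player-picked ground spot into the air.
; After cooldown and cost checks, it enables caster aim mode and plays a montage while a BP_GATargetActor_GroundPick target actor awaits confirmation.
; On confirm, it commits, plays the cast montage, launches targeted characters upward and applies GE_UpperCut_FinalBlow to them.
; Cancellation or interruption while aiming ends the ability, and ending switches aim mode off.
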(event `self.K2_ActivateAbility`
  (bind _castam_task (`self.CastAM_Task`))
  (`parent.K2_ActivateAbility`)
  (bind _returnvalue (`self.K2_CheckAbilityCooldown`))
  (if _returnvalue
    (bind _returnvalue_2 (`self.K2_CheckAbilityCost`))
    (if _returnvalue_2
      (`self.SetCasterAimMode` true)
      (bind _asynctaskproxy (`AbilityTask_PlayMontageAndWait.CreatePlayMontageAndWaitProxy` "None" "/Game/Blueprints/Player/GAS/GroundBlast/AM_GroundBlast.AM_GroundBlast")
        (:`then`
          (set `self.CastAM_Task` _asynctaskproxy)
          (add `AbilityTask_PlayMontageAndWait.OnBlendOut` _asynctaskproxy (delegate `End`))
          (add `AbilityTask_PlayMontageAndWait.OnCancelled` _asynctaskproxy (delegate `End`))
          (add `AbilityTask_PlayMontageAndWait.OnInterrupted` _asynctaskproxy (delegate `End`))
          (bind (_asynctaskproxy_2 _data) (`AbilityTask_WaitTargetData.WaitTargetData` "None" "UserConfirmed" "/Game/Blueprints/Player/GAS/GroundBlast/BP_GATargetActor_GroundPick.BP_GATargetActor_GroundPick_C" (struct) (struct) null)
            (:`ValidData`
              (clear `AbilityTask_PlayMontageAndWait.OnBlendOut` _castam_task)
              (clear `AbilityTask_PlayMontageAndWait.OnCancelled` _castam_task)
              (clear `AbilityTask_PlayMontageAndWait.OnInterrupted` _castam_task)
              (`self.K2_CommitAbility`)
              (`AbilityTask_PlayMontageAndWait.CreatePlayMontageAndWaitProxy` "None" "/Game/Blueprints/Player/GAS/GroundBlast/AM_GroundBlast_Cast.AM_GroundBlast_Cast"
                (:`then`
                  (`self.LaunchActorsFromTargetData` _data (`self.UpBlastLaunchSpeed`))
                  (`self.BP_ApplyGameplayEffectToTarget` _data "/Game/Blueprints/Player/GAS/UpperCut/Effects/FinalBlow/GE_UpperCut_FinalBlow.GE_UpperCut_FinalBlow_C"))
                (:`OnCompleted`
                  (`self.K2_EndAbility` :!label _label))
                (:`OnBlendOut`
                  (goto _label))
                (:`OnInterrupted`
                  (goto _label))
                (:`OnCancelled`
                  (goto _label))))
            (:`Cancelled`
              (`self.K2_EndAbility`))))))))

(event `End`
  (`self.K2_EndAbility`))

(event `self.K2_OnEndAbility`
  (params (bWasCancelled :type Boolean))
  (`self.SetCasterAimMode` false))

(event `SetCasterAimMode`
  (params (bInAimMode :type Boolean))
  (`CTCharacterBase.SetEanbleAiming` (`self.GetAvatarAsCTCharacter`) bInAimMode))

(event `LaunchActorsFromTargetData`
  (params (TargetData :type "GameplayAbilityTargetDataHandle Structure (by ref)") (LaunchSpeed :type "Float (single-precision)"))
  (for _array_element (`AbilitySystemBlueprintLibrary.GetActorsFromTargetData` TargetData)
    (`self.LaunchActorAsCharacter` _array_element LaunchSpeed)))

(event `LaunchActorAsCharacter`
  (params (Actor :type "Actor Object Reference") (LaunchSpeed :type "Float (single-precision)"))
  (bind _ascharacter (cast `Character` Actor))
  (`Character.LaunchCharacter` _ascharacter (* LaunchSpeed (`KismetMathLibrary.Vector_Up`)) true true))