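; GA_Dash is a gameplay ability that launches the avatar forward while playing a dash montage, with walk speed zeroed until the ability ends.
; Montage gameplay events time the dash: DashStart applies a velocity impulse and binds capsule hit detection, DashStop unbinds it.
; Hostile actors hit receive a damage-style GE_DashHit effect and are pushed along the dash direction, with separate air and ground impulse speeds.
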(event `self.K2_ActivateAbility`
  (bind _returnvalue (`Actor.GetComponentByClass` (`self.GetAvatarActorFromActorInfo`) "/Script/Engine.CharacterMovementComponent"))
  (bind _returnvalue_2 (`self.K2_CommitAbility`))
  (if _returnvalue_2
    (set `self.Max Walk Speed` (`CharacterMovementComponent.MaxWalkSpeed` _returnvalue))
    (set `CharacterMovementComponent.MaxWalkSpeed` 0.0 _returnvalue)
    (`AbilityTask_PlayMontageAndWait.CreatePlayMontageAndWaitProxy` "None" "/Game/Blueprints/Player/GAS/Dash/AM_Dash.AM_Dash"
      (:`then`
        (`AbilityTask_WaitGameplayEvent.WaitGameplayEvent` (struct :`TagName` "Ability.Dash.DashStart") null
          (:`then`
            (`AbilityTask_WaitGameplayEvent.WaitGameplayEvent` (struct :`TagName` "Ability.Dash.DashStop") null
              (:`EventReceived`
                (`self.StopHitDetection`))))
          (:`EventReceived`
            (`self.Push`)
            (`self.Start hitDetection`))))
      (:`OnCompleted`
        (`self.K2_EndAbility` :!label _label))
      (:`OnBlendOut`
        (goto _label))
      (:`OnInterrupted`
        (goto _label))
      (:`OnCancelled`
        (goto _label)))))

(event `self.K2_OnEndAbility`
  (params (bWasCancelled :type Boolean))
  (set `CharacterMovementComponent.MaxWalkSpeed` (`self.Max Walk Speed`) (`Actor.GetComponentByClass` (`self.GetAvatarActorFromActorInfo`) "/Script/Engine.CharacterMovementComponent")))

(event `Start hitDetection`
  (add `PrimitiveComponent.OnComponentHit` (`Actor.GetComponentByClass` (`self.GetAvatarActorFromActorInfo`) "/Script/Engine.CapsuleComponent") (delegate `Hit`)))

(event `Push`
  (bind _returnvalue (`self.GetAvatarActorFromActorInfo`))
  (`self.PushActor` _returnvalue (`Actor.GetActorForwardVector` _returnvalue) (`self.DashAirSpeed`) (`self.DashGroundSpeed`)))

(event `Hit`
  (params (HitComponent :type "PrimitiveComponent Object Reference") (OtherActor :type "Actor Object Reference") (OtherComp :type "PrimitiveComponent Object Reference") (NormalImpulse :type "Vector Structure") (Hit :type "HitResult Structure (by ref)"))
  (if (`self.IsOtherHostile` OtherActor)
    (`self.BP_ApplyGameplayEffectToTarget` (`AbilitySystemBlueprintLibrary.AbilityTargetDataFromActor` OtherActor) "/Game/Blueprints/Player/GAS/Dash/GE_DashHit.GE_DashHit_C")
    (`self.PushActor` OtherActor (`Actor.GetActorForwardVector` (`self.GetAvatarActorFromActorInfo`)) (`self.AirPushSpeed`) (`self.GroundPushSpeed`))))

(event `StopHitDetection`
  (remove `PrimitiveComponent.OnComponentHit` (`Actor.GetComponentByClass` (`self.GetAvatarActorFromActorInfo`) "/Script/Engine.CapsuleComponent") (delegate `Hit`)))

(fn `PushActor`
  (params (ActorToPush :type "Actor Object Reference") (PushDir :type "Vector Structure") (AirPushSpeed :type "Float (double-precision)") (GroundPushSpeed :type "Float (double-precision)"))
  (locals (ActorMovementComp :type "CharacterMovementComponent Object Reference") (PushDirection :type "Vector Structure" :default (0.0 0.0 0.0)))
  (set `local.PushDirection` (`KismetMathLibrary.Normal` PushDir))
  (bind _ascharacter (cast `Character` ActorToPush))
  (bind _output_get (set `local.ActorMovementComp` (`Character.CharacterMovement` _ascharacter)))
  (if (`NavMovementComponent.IsFalling` _output_get)
    (`CharacterMovementComponent.AddImpulse` (`local.ActorMovementComp`) (* (`local.PushDirection`) AirPushSpeed) true)
    (else
      (`CharacterMovementComponent.AddImpulse` (`local.ActorMovementComp`) (* (`local.PushDirection`) GroundPushSpeed) true))))