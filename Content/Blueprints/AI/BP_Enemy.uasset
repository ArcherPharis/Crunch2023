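; Enemy Blueprint built on the Gameplay Ability System, with a health bar, loot drop and EXP reward.
; On BeginPlay it caches its ValueGauge widget, which HealthUpdated refreshes, then activates GA_TestConfirm after a short delay.
; OnDeath spawns a random class from EffectPickup at the enemy's transform.
; AwardEXP grants experience by applying the EXPReward gameplay effect to the first player's ability system.
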(event `self.ReceiveBeginPlay`
  (`parent.ReceiveBeginPlay`)
  (bind _asvalue_gauge (cast `/Game/Blueprints/Widgets/ValueGauge` (`WidgetComponent.GetUserWidgetObject` (`self.Widget`))))
  (set `self.HealthBar` _asvalue_gauge)
  (`KismetSystemLibrary.Delay` 0.2)
  (`AbilitySystemComponent.TryActivateAbilityByClass` (`AbilitySystemBlueprintLibrary.GetAbilitySystemComponent` self) "/Game/Blueprints/Player/GAS/TestAbility/GA_TestConfirm.GA_TestConfirm_C" true))

(event `self.BP_HealthUpdated`
  (params (Health :type "Float (single-precision)") (HealthDelta :type "Float (single-precision)") (maxHealth :type "Float (single-precision)"))
  (bind _healthbar (`self.HealthBar`))
  (`/Engine/EditorBlueprintResources/StandardMacros.IsValid` _healthbar
    (:`Is Valid`
      (`/Game/Blueprints/Widgets/ValueGauge.SetValue` _healthbar Health maxHealth))))

(event `self.BP_OnDeath`
  (bind _effectpickup (`self.EffectPickup`))
  (`|SpawnActorFromClass` (`|GetArrayItem` _effectpickup (`KismetMathLibrary.RandomInteger` (`KismetArrayLibrary.Array_Length` _effectpickup))) (`self.GetTransform`) "Undefined" "OverrideRootScale" null null))

(event `self.AwardEXP`
  (`AbilitySystemComponent.BP_ApplyGameplayEffectToTarget` :`self` (`AbilitySystemBlueprintLibrary.GetAbilitySystemComponent` self) :`GameplayEffectClass` (`self.EXPReward`) :`Target` (`AbilitySystemBlueprintLibrary.GetAbilitySystemComponent` (`GameplayStatics.GetPlayerCharacter` 0))))

(fn `UserConstructionScript`
  (`parent.UserConstructionScript`))